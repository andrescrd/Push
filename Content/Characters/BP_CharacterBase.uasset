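; Base character Blueprint that supplies shared death and sound reactions for characters with a health component.
; OnDie disables character movement and turns on mesh physics simulation for a ragdoll-style death.
; OnPush and OnChangePssees each play a 2D sound.
; BeginPlay and the health-changed event are empty, and the logic for creating and updating a lives widget is left disconnected.
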(event OnHealthChanged(HealthComp)
  (params (HealthComp :type P%20Health%20Component%20Object%20Reference) (Lifes :type Integer) (DamageType :type Damage%20Type%20Object%20Reference) (InstigatedBy :type Controller%20Object%20Reference) (DamageCauser :type Actor%20Object%20Reference)))

(event EventOnDie
  (Pawn|Components|CharacterMovement|DisableMovement (Variables|Character|GetCharacterMovement))
  (Physics|SetSimulatePhysics (Variables|Character|GetMesh) true))

(event EventBeginPlay)

(event EventOnPush
  (Audio|PlaySound2D "/Game/Sounds/Sounds/UI/Laser_Push.Laser_Push" 1.0 1.0 0.0 0 0))

(event EventOnChangePssees
  (Audio|PlaySound2D "/Game/Sounds/Sounds/UI/Leave_Simulate.Leave_Simulate" 1.0 1.0 0.0 0 0))

(fn ConstructionScript)