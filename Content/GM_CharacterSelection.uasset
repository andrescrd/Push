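; Game mode for the front end, which runs the flow from main menu through level choice to character selection and game start.
; Setting a level stores it in the game instance and opens the selection widget in cinematic mode with a cursor.
; Left/right moves a clamped index across three characters, with a timeline lerping the player pawn and control rotation to each preset transform.
; Starting saves the chosen class and loads the level through the level manager.
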(event Custom|SetSelectedLevel
  (params (Level :type Integer))
  ;[0 0.2109 1] Setup level selected
  (bind _returnvalue (Class|PBlueprintFunctionLibrary|GetOwnGameInstance self))
  (Class|PGameInstance|SetLevel _returnvalue Level)
  (CallFunction|SelectCharacter))

(event Custom|MoveRight
  ;[0.6839 1 0.0478] Move next and previous character selection
  (bind _output_get (Variables|Default|SetCharacterSelected (Math|Integer|Clamp(Integer) (+ (Variables|Default|GetCharacterSelected) 1) 0 2)))
  (CallFunction|UpdatePosition _output_get))

(event Custom|UpdateTransform
  (params (Transform :type Transform) (Alpha :type Float%20%28single-precision%29))
  ;[0 1 0.351] Update position for character selected
  (bind _alpha (Timeline|Timeline_2 PlayFromStart)
    (:Update
      (Transformation|SetActorTransform (Game|Player|GetPlayerPawn 0) (Math|Transform|MakeTransform (.location (Math|Transform|Lerp(Transform) (Transformation|GetActorTransform (Game|Player|GetPlayerPawn 0)) Transform _alpha)) (.rotation (Math|Transform|Lerp(Transform) (Transformation|GetActorTransform (Game|Player|GetPlayerPawn 0)) Transform _alpha)) "1,1,1"))
      (Pawn|SetControlRotation (Game|GetPlayerController 0) (.rotation (Math|Transform|Lerp(Transform) (Transformation|GetActorTransform (Game|Player|GetPlayerPawn 0)) Transform _alpha))))))

(event Custom|UpdatePosition
  (params (Index :type Integer))
  ;[0 1 0.351] Update position for character selected
  (switch int Index
    (:0
      (CallFunction|UpdateTransform (Variables|Default|GetPigPosition) 0.0))
    (:1
      (CallFunction|UpdateTransform (Variables|Default|GetWoodPosition) 0.0))
    (:2
      (CallFunction|UpdateTransform (Variables|Default|GetMooshroomPosition) 0.0))))

(event Custom|StartGame
  ;[1 0.04044 0] Start play after level and character selection
  (bind _returnvalue (Class|PBlueprintFunctionLibrary|GetOwnGameInstance self))
  (bind _newparam (CallFunction|GetCharacterSelectedClass))
  (Class|PGameInstance|SetPlayerClass _returnvalue _newparam)
  (bind _returnvalue_2 (Class|PGameInstance|GetPlayerSetup _returnvalue))
  (bind _returnvalue_3 (Class|PBlueprintFunctionLibrary|GetLevelManager self))
  (bind _returnvalue_4 (Class|PLevelManager|GetLevels _returnvalue_3))
  (Class|PLevelManager|LoadLevel _returnvalue_3 self (.levelname (Utilities|Array|Get(acopy) _returnvalue_4 (.level _returnvalue_2)))))

(event Custom|MoveLeft
  ;[0.6839 1 0.0478] Move next and previous character selection
  (bind _output_get (Variables|Default|SetCharacterSelected (Math|Integer|Clamp(Integer) (- (Variables|Default|GetCharacterSelected) 1) 0 2)))
  (CallFunction|UpdatePosition _output_get))

(event Custom|SelectCharacter
  ;[1 0.5264 0.3345] Open character sleection
  (Viewport|RemoveAllWidgets)
  (bind _returnvalue (UserInterface|CreateWidget "/Game/UI/SelectCharacterWidget.SelectCharacterWidget_C" (Game|GetPlayerController 0) 0))
  (UserInterface|Viewport|AddtoViewport _returnvalue 0)
  (CallFunction|UpdatePosition)
  (Class|PlayerController|SetCinematicMode (Game|GetPlayerController 0) true true true true true)
  (Variables|/Script/Engine.PlayerController|SetbShowMouseCursor (Game|GetPlayerController 0) true))

(event EventBeginPlay
  ;[1 0 0.8129] Set Main Menu
  (bind _returnvalue (UserInterface|CreateWidget "/Game/UI/MainMenu.MainMenu_C"))
  (UserInterface|Viewport|AddtoViewport _returnvalue 0))

(fn ConstructionScript)

(fn GetCharacterSelectedClass
  (return (Utilities|Select :Index (Variables|Default|GetCharacterSelected) :Option%200 "/Game/Characters/BP_Pig.BP_Pig_C" :Option%201 "/Game/Characters/BP_Wood.BP_Wood_C" :Option%202 "/Game/Characters/BP_Mushroom.BP_Mushroom_C")))