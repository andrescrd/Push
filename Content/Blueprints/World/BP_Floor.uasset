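; BP_Floor is a physics floor that reacts to the positions of characters, tilting within a limited range.
; Every tick it finds all Characters and applies a vertical force to its static mesh at each one's XY position, at the floor's height.
; It then slowly interpolates its rotation toward a copy with roll, pitch and yaw each clamped to the MaxRotation range, softly limiting the tilt.
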(event EventTick
  (params (DeltaSeconds :type Float%20%28single-precision%29))
  (bind _returnvalue (Transformation|GetActorRotation))
  (bind _maxrotation (Variables|Default|GetMaxRotation))
  (Utilities|FlowControl|Sequence
    (:then_0
      (bind _outactors (Actor|GetAllActorsOfClass "/Script/Engine.Character"))
      (for _array_element _outactors
        (bind _ascharacter (Utilities|Casting|CastToCharacter _array_element))
        (Class|PrimitiveComponent|AddForceatLocation (Variables|Debug|GetStaticMeshComponent) (Math|Vector|MakeVector 0.0 0.0 (Variables|Default|GetForce)) (Math|Vector|MakeVector (.x (Transformation|GetActorLocation _ascharacter)) (.y (Transformation|GetActorLocation _ascharacter)) (.z (Transformation|GetActorLocation))) "None")))
    (:then_1
      (Transformation|SetActorRotation (Math|Interpolation|RInterpTo (Transformation|GetActorRotation) (Math|Rotator|MakeRotator (Math|Float|Clamp(Float) (.roll _returnvalue) (.value (.lowerbound _maxrotation)) (.value (.upperbound _maxrotation))) (Math|Float|Clamp(Float) (.pitch _returnvalue) (.value (.lowerbound _maxrotation)) (.value (.upperbound _maxrotation))) (Math|Float|Clamp(Float) (.yaw _returnvalue) (.value (.lowerbound _maxrotation)) (.value (.upperbound _maxrotation)))) (Utilities|Time|GetWorldDeltaSeconds) 0.3)))))

(fn ConstructionScript)