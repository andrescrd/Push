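; World spawner that populates the level with randomly chosen Wood, Pig and Mushroom actors and relocates living characters on request.
; On BeginPlay it runs one EQS_FindSpawnLocation query per bot in the game mode's MaxNumberOfBots, picking from the best 25%.
; Query results become spawn points, and spawned Characters have movement disabled.
; RespawmActor reruns the query for all matches, then teleports the living PCharacter slightly above the first result.
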(event Custom|RespawmActor
  (params (Actor :type Actor%20Object%20Reference))
  (bind _output_get (Variables|Default|SetCurrentActor Actor))
  (bind _aspcharacter (Utilities|Casting|CastToPCharacter _output_get))
  (bind _returnvalue (Class|PCharacter|GetIsAlive _aspcharacter))
  (if _returnvalue
    (bind _returnvalue_2 (AI|EQS|RunEQSQuery "/Game/AI/EQS/EQS_FindSpawnLocation.EQS_FindSpawnLocation" self "AllMatching"))
    (EventDispatchers|BindEventtoOnQueryFinishedEvent _returnvalue_2 (delegate Custom|CustomEvent))))

(event Custom|SpawnActor
  (bind _returnvalue (AI|EQS|RunEQSQuery "/Game/AI/EQS/EQS_FindSpawnLocation.EQS_FindSpawnLocation" self "RandomBest25Pct"))
  (EventDispatchers|BindEventtoOnQueryFinishedEvent _returnvalue (delegate Custom|OnEQSFinished)))

(event Custom|OnEQSFinished
  (params (QueryInstance :type Env%20Query%20Instance%20Blueprint%20Wrapper%20Object%20Reference) (QueryStatus :type EEnvQueryStatus%20Enum :default "Processing"))
  (switch Utilities|FlowControl|Switch|SwitchonEEnvQueryStatus QueryStatus
    (:Success
      (bind _resultlocations (AI|EQS|GetQueryResultsasLocations QueryInstance))
      (for _array_element _resultlocations
        (bind _returnvalue (Game|SpawnActorfromClass (Utilities|Select :Index (Math|Random|RandomIntegerinRange 0 2) :Option%200 "/Game/Characters/BP_Wood.BP_Wood_C" :Option%201 "/Game/Characters/BP_Pig.BP_Pig_C" :Option%202 "/Game/Characters/BP_Mushroom.BP_Mushroom_C") (Math|Transform|MakeTransform _array_element) "AdjustIfPossibleButDontSpawnIfColliding" 0 0))
        (bind _ascharacter (Utilities|Casting|CastToCharacter _returnvalue))
        (Pawn|Components|CharacterMovement|DisableMovement (Variables|/Script/Engine.Character|GetCharacterMovement _ascharacter))))))

(event Custom|CustomEvent
  (params (QueryInstance :type Env%20Query%20Instance%20Blueprint%20Wrapper%20Object%20Reference) (QueryStatus :type EEnvQueryStatus%20Enum :default "Processing"))
  (switch Utilities|FlowControl|Switch|SwitchonEEnvQueryStatus QueryStatus
    (:Success
      (bind _resultlocations (AI|EQS|GetQueryResultsasLocations QueryInstance))
      (Components|Movement|StopMovementImmediately (Actor|GetComponentbyClass (Variables|Default|GetCurrentActor) "/Script/Engine.CharacterMovementComponent"))
      (Transformation|SetActorLocation (Variables|Default|GetCurrentActor) (Math|Vector|MakeVector (.x (Utilities|Array|Get(acopy) _resultlocations)) (.y (Utilities|Array|Get(acopy) _resultlocations)) (+ (.z (Utilities|Array|Get(acopy) _resultlocations)) 1e+02)) false true))))

(event EventBeginPlay
  (for _index (range 1 (Variables|/Script/Push.PGameMode|GetMaxNumberOfBots (.AsPGame%20Mode (Utilities|Casting|CastToPGameMode (Game|GetGameMode)))))
    (CallFunction|SpawnActor)))

(fn ConstructionScript)