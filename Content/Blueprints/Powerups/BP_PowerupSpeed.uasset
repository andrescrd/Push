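; Speed powerup Blueprint that temporarily doubles the walk speed of the Character that activates it.
; On activation it stores the Character, hides its mesh and sets MaxWalkSpeed to twice the movement component's current GetMaxSpeed.
; On expiry it halves the current max speed rather than restoring a saved value, then destroys itself.
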(event EventOnActivated
  (params (ActivatorActor :type Actor%20Object%20Reference))
  (bind _ascharacter (Utilities|Casting|CastToCharacter ActivatorActor))
  (Variables|Default|SetActivatorRef _ascharacter)
  (Rendering|SetVisibility (Variables|Default|GetStaticMesh) false true)
  (Variables|/Script/Engine.CharacterMovementComponent|SetMaxWalkSpeed (Actor|GetComponentbyClass (Variables|Default|GetActivatorRef) "/Script/Engine.CharacterMovementComponent") (* (Class|MovementComponent|GetMaxSpeed (Actor|GetComponentbyClass (Variables|Default|GetActivatorRef) "/Script/Engine.CharacterMovementComponent")) 2.0)))

(event EventOnExpired
  (bind _activatorref (Variables|Default|GetActivatorRef))
  (bind _returnvalue (Actor|GetComponentbyClass _activatorref "/Script/Engine.CharacterMovementComponent"))
  (Variables|/Script/Engine.CharacterMovementComponent|SetMaxWalkSpeed _returnvalue (/ (Class|MovementComponent|GetMaxSpeed _returnvalue) 2.0))
  (Actor|DestroyActor))

(fn ConstructionScript)